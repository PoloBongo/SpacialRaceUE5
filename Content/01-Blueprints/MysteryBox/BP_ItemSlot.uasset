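; BP_ItemSlot holds the player's current power-up and spends it when B is pressed.
; On BeginPlay it creates the WG_PowerUP widget and adds it to the viewport.
; B switches on SlotItem: the first ability prints and deducts LaserNbUse from ItemUse, while the other two only print debug text.
; CheckPowerUP then empties the slot and refreshes the widget once ItemUse is depleted.
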(event Custom|CheckPowerUP
  (if (<= (Variables|Default|GetItemUse) 0.001)
    (Variables|Default|SetSlotItem 0)
    (Default|UpdUI (Variables|Default|GetUIpowerUp))))

(event EventBeginPlay
  ;[1 1 1] Création du widget
  (bind _returnvalue (UserInterface|CreateWidget "/Game/05-UI/WG_PowerUP.WG_PowerUP_C"))
  (UserInterface|Viewport|AddtoViewport _returnvalue 0)
  (Variables|Default|SetUIpowerUp _returnvalue))

(event Input|KeyboardEvents|B
  (params (Key :type Key%20Structure :default "None"))
  (:Pressed
    (switch int (Variables|Default|GetSlotItem)
      (:1
        (Development|PrintString "Capacité 1")
        (Variables|Default|SetItemUse (- (Variables|Default|GetItemUse) (Variables|Default|GetLaserNbUse)))
        (CallFunction|CheckPowerUP))
      (:2
        (Development|PrintString "Capacité 2"))
      (:3
        (Development|PrintString "Capacité 3")))))

(fn ConstructionScript)