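; BP_MysteryBox is a pickup box that grants a random power-up to the player's hover vehicle.
; On BeginPlay it caches the first BP_ItemSlot actor found in the level, rather than a slot taken from the overlapping actor.
; When a BP_HoverController overlaps the box and that slot is empty, it rolls an item, sets its use value, refreshes the power-up UI and destroys itself.
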(event OnComponentBeginOverlap(Box)
  (params (OverlappedComponent :type Primitive%20Component%20Object%20Reference) (OtherActor :type Actor%20Object%20Reference) (OtherComp :type Primitive%20Component%20Object%20Reference) (OtherBodyIndex :type Integer) (bFromSweep :type Boolean) (SweepResult :type Hit%20Result%20Structure%20%28by%20ref%29))
  (bind _reftoitem (Variables|Default|GetRefToItem))
  ;[1 1 1] Quand le joueur rentre dans la box
  (Utilities|Casting|CastToBP_HoverController OtherActor)
  ;;[1 1 1] Vérification si le joueur à déjà un item
  (if (== (Variables|/Game/01-Blueprints/MysteryBox/BP_ItemSlot.BP_ItemSlot_C|GetSlotItem (Variables|Default|GetRefToItem)) 0)
    ;;[1 1 1] Pick un PowerUp aléatoire, update UI et destroy du cube
    (Variables|/Game/01-Blueprints/MysteryBox/BP_ItemSlot.BP_ItemSlot_C|SetSlotItem (Variables|Default|GetRefToItem) (Math|Random|RandomIntegerinRange 1 5))
    (Variables|/Game/01-Blueprints/MysteryBox/BP_ItemSlot.BP_ItemSlot_C|SetItemUse _reftoitem 1.0)
    (Default|UpdUI (Variables|/Game/01-Blueprints/MysteryBox/BP_ItemSlot.BP_ItemSlot_C|GetUIpowerUp _reftoitem))
    (Actor|DestroyActor)))

(event EventBeginPlay
  ;[1 1 1] RefToItem
  (bind _returnvalue (Actor|GetActorOfClass "/Game/01-Blueprints/MysteryBox/BP_ItemSlot.BP_ItemSlot_C"))
  (Variables|Default|SetRefToItem _returnvalue))

(fn ConstructionScript)