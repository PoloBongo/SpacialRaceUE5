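; BP_TurretTest is a turret that aims and fires at the hover player when its PawnSensing component sees it.
; Each sighting snaps the turret top's world rotation toward the player, measured from the turret's root.
; A two-second Delay then spawns a BP_TurretBullets at the Arrow's transform, which also throttles fire because repeat sightings during the wait are ignored by the Delay.
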(event OnSeePawn(PawnSensing)
  (params (Pawn :type Pawn%20Object%20Reference))
  (Utilities|Casting|CastToBP_HoverPlayer Pawn)
  (Transformation|SetWorldRotation (Variables|Default|GetBP_Turret_Top) (Math|Rotator|FindLookatRotation (Transformation|GetWorldLocation (Variables|Default|GetDefaultSceneRoot)) (Transformation|GetActorLocation Pawn)) false false)
  (Utilities|FlowControl|Delay 2.0)
  (Game|SpawnActorfromClass "/Game/01-Blueprints/Turret/BP_TurretBullets.BP_TurretBullets_C" (Transformation|GetWorldTransform (Variables|Default|GetArrow)) "AlwaysSpawn" "MultiplyWithRoot" 0 0))

(fn ConstructionScript)