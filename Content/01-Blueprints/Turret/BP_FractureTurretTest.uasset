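; BP_FractureTurretTest is a test turret that aims and fires at the hover-controlled player pawn it sees.
; When PawnSensing spots a BP_HoverController, the GCBPTurretTop component snaps to face that pawn from the turret root.
; After a short delay, it spawns a BP_TurretBullets actor at the Arrow component's transform, with no other firing loop or state.
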(event OnSeePawn(PawnSensing)
  (params (Pawn :type Pawn%20Object%20Reference))
  (Utilities|Casting|CastToBP_HoverController Pawn)
  (Transformation|SetWorldRotation (Variables|Default|GetGC_BP_Turret_Top) (Math|Rotator|FindLookatRotation (Transformation|GetWorldLocation (Variables|Default|GetDefaultSceneRoot)) (Transformation|GetActorLocation Pawn)) false false)
  (Utilities|FlowControl|Delay 1.0)
  (Game|SpawnActorfromClass "/Game/01-Blueprints/Turret/BP_TurretBullets.BP_TurretBullets_C" (Transformation|GetWorldTransform (Variables|Default|GetArrow)) "Undefined" "MultiplyWithRoot" 0 0))

(fn ConstructionScript)