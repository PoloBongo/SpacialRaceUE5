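; BP_FractureTurret is a destructible turret that shoots at the player's BP_HoverController.
; After a startup delay it caches that actor, then on Tick, while it is in range, aims the top at it.
; A Delay on Tick paces the BP_TurretBullets spawned from the Arrow, with a laser sound.
; A Chaos break on the bottom geometry collection plays an explosion, changes collision type, stops firing and later destroys the actor.
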(event OnChaosBreakEvent(GC_BP_Turret_Bot)
  (params (BreakEvent :type Chaos%20Break%20Event%20Structure%20%28by%20ref%29))
  (Audio|SpawnSoundatLocation "/Game/07-Sounds/large-underwater-explosion-190270.large-underwater-explosion-190270" (Transformation|GetActorLocation) "0, 0, 0" 0.2 1.0 0.0 0 0)
  (Collision|SetCollisionObjectType (Variables|Default|GetGC_BP_Turret_Top) "ECC_GameTraceChannel2")
  (Variables|Default|SetIsDestroy true)
  (Utilities|FlowControl|Delay 1e+01)
  (Actor|DestroyActor))

(event EventTick
  (params (DeltaSeconds :type Float%20%28single-precision%29))
  (bind _refhovercontroller (Variables|Default|GetRefHoverController))
  (bind _meshescomponents (Variables|/Script/RacersProject_UE5.HoverController|GetMeshesComponents _refhovercontroller))
  (bind _output (Utilities|Array|Get(acopy) _meshescomponents))
  (bind _returnvalue (Transformation|GetWorldLocation _output))
  ;[1 1 1] Récupération de Main 0
  (Utilities|IsValid _refhovercontroller
    (:Is%20Valid
      ;[1 1 1] Vérification distance entre le joueur et la tourelle
      (Variables|Default|SetPlayerinRange (<= (Math|Vector|VectorLength (- (Transformation|GetActorLocation) _returnvalue)) (Variables|Default|GetDistTurretToPlayer)))
      (if (Variables|Default|GetPlayerinRange)
        ;[1 1 1] Rotation et Tir la tourelle
        (Transformation|SetWorldRotation (Variables|Default|GetGC_BP_Turret_Top) (Math|Rotator|FindLookatRotation (Transformation|GetWorldLocation (Variables|Default|GetDefaultSceneRoot)) _returnvalue) false false)
        (Utilities|FlowControl|Delay 2.0)
        (if (not (Variables|Default|GetIsDestroy))
          (bind _returnvalue_2 (Game|SpawnActorfromClass "/Game/01-Blueprints/Turret/BP_TurretBullets.BP_TurretBullets_C" (Transformation|GetWorldTransform (Variables|Default|GetArrow)) "Undefined" "MultiplyWithRoot" 0 0))
          (Audio|PlaySoundatLocation "/Game/07-Sounds/laser-zap-90575.laser-zap-90575" (Transformation|GetActorLocation _returnvalue_2) "0, 0, 0" 0.2 1.0 0.0 0 0 0 0))))))

(event EventBeginPlay
  (Utilities|FlowControl|Delay 3.0)
  (bind _returnvalue (Actor|GetActorOfClass "/Game/01-Blueprints/Hover/BP_HoverController.BP_HoverController_C"))
  (Variables|Default|SetRefHoverController _returnvalue)
  (bind _returnvalue_2 (Actor|GetActorOfClass "/Game/01-Blueprints/Turret/BP_SpawnLocation.BP_SpawnLocation_C"))
  (Variables|Default|SetRefTgPoint _returnvalue_2)
  (Variables|Default|SetIsDestroy false))

(fn ConstructionScript)