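; Hover suspension component that pushes the BP_HoverController's physics body away from the surface beneath it.
; Each tick it traces along its negative up vector and converts compression into a spring-damper force, using the controller's stiffness and damping, applied at its location on static mesh hits.
; Hitting a BP_SplineTool_Tiedtke_Deformation actor turns on the controller's wall-ride flag and flips its angular rotation speed negative; other hits restore both.
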(event EventBeginPlay
  (bind _returnvalue (Actor|GetActorOfClass "/Game/01-Blueprints/Hover/BP_HoverController.BP_HoverController_C"))
  (bind _output_get (Variables|Default|SetBP_HoverController _returnvalue))
  (bind _output_get_2 (Variables|Default|SetRefToBody (Utilities|Array|Get(acopy) (Variables|/Script/RacersProject_UE5.HoverController|GetMeshesComponents _output_get))))
  (if (not (Physics|IsSimulatingPhysics _output_get_2 "None"))
    (Variables|Default|SetRefToBody 0)))

(event EventTick
  (params (DeltaSeconds :type Float%20%28single-precision%29))
  (bind _returnvalue (Transformation|GetWorldLocation))
  (bind _bp_hovercontroller (Variables|Default|GetBP_HoverController))
  (bind _distancebetweenhovertoground (Variables|Default|GetDistanceBetweenHoverToGround))
  (Variables|Default|GetRefToBody
    (:then
      (bind (_outhit _returnvalue_2) (Collision|LineTraceByChannel _returnvalue (- _returnvalue (* (Math|Vector|GetUpVector) (Variables|Default|GetDistanceBetweenHoverToGround))) "TraceTypeQuery1" false (Utilities|Array|MakeArray (Components|GetOwner)) (select (Variables|Default|GetDebugLineTrace) "ForOneFrame" "None")))
      (if _returnvalue_2
        (Utilities|FlowControl|Sequence
          (:then_0
            (Utilities|Casting|CastToStaticMeshComponent (.HitComponent (Collision|BreakHitResult _outhit)))
            (Variables|Default|SetHoverForce (+ (* (/ (- (/ (- _distancebetweenhovertoground (.Distance (Collision|BreakHitResult _outhit))) _distancebetweenhovertoground) (Variables|Default|GetPreviousCompression)) (Utilities|Time|GetWorldDeltaSeconds)) (Variables|/Script/RacersProject_UE5.HoverController|GetDamping (Variables|Default|GetBP_HoverController))) (* (/ (- _distancebetweenhovertoground (.Distance (Collision|BreakHitResult _outhit))) _distancebetweenhovertoground) (Variables|/Script/RacersProject_UE5.HoverController|GetStifness (Variables|Default|GetBP_HoverController)))))
            (Variables|Default|SetPreviousCompression (/ (- _distancebetweenhovertoground (.Distance (Collision|BreakHitResult _outhit))) _distancebetweenhovertoground))
            (Class|PrimitiveComponent|AddForceatLocation (Variables|Default|GetRefToBody) (* (Math|Vector|GetUpVector) (Variables|Default|GetHoverForce)) (Transformation|GetWorldLocation) "None"))
          (:then_1
            (Utilities|Casting|CastToBP_SplineTool_Tiedtke_Deformation (.HitActor (Collision|BreakHitResult _outhit))
              (:then
                (Variables|/Script/RacersProject_UE5.HoverController|SetAngularRotSpeed _bp_hovercontroller -1e+02)
                (Variables|/Game/01-Blueprints/Hover/BP_HoverController.BP_HoverController_C|SetIsWallRide _bp_hovercontroller true))
              (:CastFailed
                (Variables|/Script/RacersProject_UE5.HoverController|SetAngularRotSpeed _bp_hovercontroller 1e+02)
                (Variables|/Game/01-Blueprints/Hover/BP_HoverController.BP_HoverController_C|SetIsWallRide _bp_hovercontroller false)))))))
    (:else
      (bind _returnvalue_3 (Actor|GetActorOfClass "/Game/01-Blueprints/Hover/BP_HoverController.BP_HoverController_C"))
      (Variables|Default|SetRefToBody (Utilities|Array|Get(acopy) (Variables|/Script/RacersProject_UE5.HoverController|GetMeshesComponents _returnvalue_3))))))