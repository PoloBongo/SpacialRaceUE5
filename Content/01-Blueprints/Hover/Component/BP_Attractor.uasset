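; BP_Attractor is a hover scene component that probes the ground and gates player input by surface type.
; It caches BP_HoverController and its first mesh, then line-traces along its down vector each Tick.
; Static mesh hits enable input; other hits disable it, set a negative movement TargetSpeed and re-enable input after a delay.
; Despite the name, it applies no attraction force.
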(event EventBeginPlay
  (bind _returnvalue (Actor|GetActorOfClass "/Game/01-Blueprints/Hover/BP_HoverController.BP_HoverController_C"))
  (bind _output_get (Variables|Default|SetBP_HoverController _returnvalue))
  (bind _output_get_2 (Variables|Default|SetRefToBody (Utilities|Array|Get(acopy) (Variables|/Script/RacersProject_UE5.HoverController|GetMeshesComponents _output_get))))
  (if (Physics|IsSimulatingPhysics _output_get_2 "None")
    _))

(event EventTick
  (params (DeltaSeconds :type Float%20%28single-precision%29))
  (bind _returnvalue (Game|Player|GetPlayerPawn 0))
  (bind _returnvalue_2 (Transformation|GetWorldLocation))
  (Variables|Default|GetRefToBody
    (:then
      (bind (_outhit _returnvalue_3) (Collision|LineTraceByChannel _returnvalue_2 (- _returnvalue_2 (* (Math|Vector|GetUpVector) (Variables|Default|GetDistanceBetweenHoverToGround))) "TraceTypeQuery1" false (Utilities|Array|MakeArray (Components|GetOwner)) (select (Variables|Default|GetDebugLineTrace) "ForOneFrame" "None")))
      (if _returnvalue_3
        (Utilities|Casting|CastToStaticMeshComponent (.HitComponent (Collision|BreakHitResult _outhit))
          (:then
            (Input|EnableInput _returnvalue 0))
          (:CastFailed
            (Input|DisableInput _returnvalue 0)
            (Variables|/Game/01-Blueprints/Hover/Component/BP_MovementComponent.BP_MovementComponent_C|SetTargetSpeed (Variables|/Game/01-Blueprints/Hover/BP_HoverController.BP_HoverController_C|GetBP_MovementComponent (Variables|Default|GetBP_HoverController)) -5e+02)
            (Utilities|FlowControl|Delay 1e+01)
            (Input|EnableInput (Game|Player|GetPlayerPawn 0) 0)))))
    (:else
      (bind _returnvalue_4 (Actor|GetActorOfClass "/Game/01-Blueprints/Hover/BP_HoverController.BP_HoverController_C"))
      (Variables|Default|SetRefToBody (Utilities|Array|Get(acopy) (Variables|/Script/RacersProject_UE5.HoverController|GetMeshesComponents _returnvalue_4))))))