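; Player-driven hover vehicle with thrust, steering, boost, flip recovery and a laser.
; Enhanced Input sets target speeds on BPMovementComponent, with boost scaling thrust and steering inverting in reverse.
; Full-rate turns shorten the inner side's hover arm distances to bank the craft, resetting on release or at low speed.
; Flip rights a tipped vehicle with timed impulses, laser spawns BP_Laser, and a scene capture renders only this actor.
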(event Custom|SetupArmLength
  (params (Length :type Float%20%28double-precision%29) (Arm :type BP%20Hover%20Component%20Object%20Reference))
  (Variables|/Game/01-Blueprints/Hover/Component/BP_HoverComponent.BP_HoverComponent_C|SetDistanceBetweenHoverToGround Arm Length))

(event Input|EnhancedActionEvents|EnhancedInputActionIA_Thrust
  (params (ActionValue :type Float%20%28double-precision%29) (ElapsedSeconds :type Float%20%28double-precision%29) (TriggeredSeconds :type Float%20%28double-precision%29) (InputAction :type Input%20Action%20Object%20Reference :default "/Game/03-Inputs/Actions/IA_Thrust.IA_Thrust"))
  (bind _bp_movementcomponent (Variables|Default|GetBP_MovementComponent))
  (:Triggered
    (Variables|/Game/01-Blueprints/Hover/Component/BP_MovementComponent.BP_MovementComponent_C|SetTargetSpeed _bp_movementcomponent (* ActionValue (Variables|Default|GetThrustSpeed) (Variables|Default|GetBoostMultiplier))))
  (:Completed
    (Variables|/Game/01-Blueprints/Hover/Component/BP_MovementComponent.BP_MovementComponent_C|SetTargetSpeed _bp_movementcomponent 0.0)))

(event Input|EnhancedActionEvents|EnhancedInputActionIA_Steer
  (params (ActionValue :type Float%20%28double-precision%29) (ElapsedSeconds :type Float%20%28double-precision%29) (TriggeredSeconds :type Float%20%28double-precision%29) (InputAction :type Input%20Action%20Object%20Reference :default "/Game/03-Inputs/Actions/IA_Steer.IA_Steer"))
  (bind _returnvalue (Input|EnhancedActionValues|GetIA_Thrust))
  (bind _bp_movementcomponent (Variables|Default|GetBP_MovementComponent))
  (:Triggered
    (bind _output_get (Variables|/Game/01-Blueprints/Hover/Component/BP_MovementComponent.BP_MovementComponent_C|SetTargetAngularSpeed _bp_movementcomponent (* ActionValue (Variables|Default|GetAngularRotSpeed) (Math|Float|SelectFloat (Math|Float|Sign(Float) _returnvalue) 1.0 (== _returnvalue 0.0)))))
    (if (== _output_get -1e+02)
      (CallFunction|ModifStabilizateurTurnLeft)
      (elif (== _output_get 1e+02)
        (CallFunction|ModifStabilizateurTurnRight))))
  (:Completed
    (Variables|/Game/01-Blueprints/Hover/Component/BP_MovementComponent.BP_MovementComponent_C|SetTargetAngularSpeed _bp_movementcomponent 0.0)
    (CallFunction|ModifStabilizateurReset)))

(event Input|EnhancedActionEvents|EnhancedInputActionIA_Flip
  (params (ActionValue :type Boolean) (ElapsedSeconds :type Float%20%28double-precision%29) (TriggeredSeconds :type Float%20%28double-precision%29) (InputAction :type Input%20Action%20Object%20Reference :default "/Game/03-Inputs/Actions/IA_Flip.IA_Flip"))
  (bind _vehicle (Variables|Default|GetVehicle))
  (bind _vehicle_2 (Variables|Default|GetVehicle))
  (if (<= (Math|Vector|DotProduct (Math|Vector|GetUpVector _vehicle) (Math|Vector|MakeVector 0.0 0.0 1.0)) 0.2)
    (Physics|AddImpulse _vehicle (* (Math|Vector|GetUpVector _vehicle) -1e+06) "None" false)
    (Utilities|FlowControl|Delay 0.2)
    (Class|PrimitiveComponent|AddAngularImpulseinDegrees _vehicle_2 (* (Math|Vector|GetForwardVector _vehicle_2) 2e+09) "None" false)))

(event Input|EnhancedActionEvents|EnhancedInputActionIA_Boost
  (params (ActionValue :type Boolean) (ElapsedSeconds :type Float%20%28double-precision%29) (TriggeredSeconds :type Float%20%28double-precision%29) (InputAction :type Input%20Action%20Object%20Reference :default "/Game/03-Inputs/Actions/IA_Boost.IA_Boost"))
  (:Ongoing
    (Variables|Default|SetBoostMultiplier 3.0))
  (:Completed
    (Variables|Default|SetBoostMultiplier 1.0)))

(event Input|EnhancedActionEvents|EnhancedInputActionIA_Laser
  (params (ActionValue :type Boolean) (ElapsedSeconds :type Float%20%28double-precision%29) (TriggeredSeconds :type Float%20%28double-precision%29) (InputAction :type Input%20Action%20Object%20Reference :default "/Game/03-Inputs/Actions/IA_Laser.IA_Laser"))
  (bind _laserspawner (Variables|Default|GetLaserSpawner))
  (Game|SpawnActorfromClass "/Game/01-Blueprints/Hover/BP_Laser.BP_Laser_C" (Math|Transform|MakeTransform (Transformation|GetWorldLocation _laserspawner) (Transformation|GetWorldRotation _laserspawner) "1.000000,1.000000,1.000000") "Undefined" "MultiplyWithRoot" 0 0))

(event EventBeginPlay
  (bind _returnvalue (Game|GetPlayerController 0))
  (bind _returnvalue_2 (PlayerController|LocalPlayerSubsystems|GetEnhancedInputLocalPlayerSubsystem _returnvalue))
  (Utilities|IsValid _returnvalue_2
    (:Is%20Valid
      (Input|AddMappingContext _returnvalue_2 "/Game/03-Inputs/IMC_Hover.IMC_Hover" 0 "(bIgnoreAllPressedKeysUntilRelease=True,bForceImmediately=False,bNotifyUserSettings=False)")
      (Rendering|SceneCapture|ShowOnlyActorComponents (Variables|Default|GetSceneCaptureComponent2D) self false))))

(event EventTick
  (params (DeltaSeconds :type Float%20%28single-precision%29))
  (if (<= (Variables|/Game/01-Blueprints/Hover/Component/BP_MovementComponent.BP_MovementComponent_C|GetCurrentSpeed (Variables|Default|GetBP_MovementComponent)) 2e+01)
    (CallFunction|ModifStabilizateurReset)))

(fn ConstructionScript)

(fn ModifStabilizateurTurnRight
  (CallFunction|SetupArmLength 3e+02 (Variables|Default|GetBL))
  (CallFunction|SetupArmLength 3e+02 (Variables|Default|GetFL))
  (CallFunction|SetupArmLength 2e+02 (Variables|Default|GetBR))
  (CallFunction|SetupArmLength 2e+02 (Variables|Default|GetFR))
  (Variables|Default|SetisTurnRight true))

(fn ModifStabilizateurTurnLeft
  (CallFunction|SetupArmLength 2e+02 (Variables|Default|GetBL))
  (CallFunction|SetupArmLength 2e+02 (Variables|Default|GetFL))
  (CallFunction|SetupArmLength 3e+02 (Variables|Default|GetBR))
  (CallFunction|SetupArmLength 3e+02 (Variables|Default|GetFR))
  (Variables|Default|SetisTurnLeft true))

(fn ModifStabilizateurReset
  (CallFunction|SetupArmLength 3e+02 (Variables|Default|GetBL))
  (CallFunction|SetupArmLength 3e+02 (Variables|Default|GetFL))
  (CallFunction|SetupArmLength 3e+02 (Variables|Default|GetBR))
  (CallFunction|SetupArmLength 3e+02 (Variables|Default|GetFR))
  (Variables|Default|SetisTurnLeft false)
  (Variables|Default|SetisTurnRight false))