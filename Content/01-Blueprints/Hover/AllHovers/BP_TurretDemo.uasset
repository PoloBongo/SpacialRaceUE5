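; Demo turret actor that moves to a spawn location and turns its top toward the BP_SpaceDemo actor in the level.
; On BeginPlay it adds both turret parts and that actor's SMVortex5 component to the show-only lists of two scene captures, CameraSpace and CameraTurret, isolating them in those views.
; After a short delay, the turret top snaps once to a look-at rotation, with no continuous tracking.
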(event EventBeginPlay
  (bind _gc_bp_turret_top (Variables|Default|GetGC_BP_Turret_Top))
  (Transformation|SetActorLocation (Variables|Default|GetSpawn) false false)
  (Rendering|SceneCapture|ShowOnlyComponent (Variables|Default|GetCameraSpace) (Variables|Default|GetGC_BP_Turret_Top))
  (Rendering|SceneCapture|ShowOnlyComponent (Variables|Default|GetCameraTurret) (Variables|Default|GetGC_BP_Turret_Top))
  (bind _returnvalue (Actor|GetActorOfClass "/Game/01-Blueprints/Hover/AllHovers/BP_SpaceDemo.BP_SpaceDemo_C"))
  (Rendering|SceneCapture|ShowOnlyComponent (Variables|Default|GetCameraTurret) (Variables|/Game/01-Blueprints/Hover/AllHovers/BP_SpaceDemo.BP_SpaceDemo_C|GetSM_Vortex_5 _returnvalue))
  (Rendering|SceneCapture|ShowOnlyComponent (Variables|Default|GetCameraSpace) (Variables|/Game/01-Blueprints/Hover/AllHovers/BP_SpaceDemo.BP_SpaceDemo_C|GetSM_Vortex_5 _returnvalue))
  (Rendering|SceneCapture|ShowOnlyComponent (Variables|Default|GetCameraSpace) (Variables|Default|GetGC_BP_Turret_Bot))
  (Rendering|SceneCapture|ShowOnlyComponent (Variables|Default|GetCameraTurret) (Variables|Default|GetGC_BP_Turret_Bot))
  (Utilities|FlowControl|Delay 5.0)
  (Transformation|SetWorldRotation _gc_bp_turret_top (Math|Rotator|FindLookatRotation (Transformation|GetWorldLocation _gc_bp_turret_top) (Transformation|GetActorLocation (Components|GetOwner (Variables|/Game/01-Blueprints/Hover/AllHovers/BP_SpaceDemo.BP_SpaceDemo_C|GetSM_Vortex_5 _returnvalue)))) false false))

(fn ConstructionScript)