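; Demo road spline actor that moves a list of actors along its spline at a fixed spacing.
; The construction script lays them out along the spline, then a Timeline started at BeginPlay drives their distance, location and rotation, skipping the transform update for any past the spline's end.
; Speed and Slow overlap volumes change the Timeline play rate when a BP_SpaceDemo enters.
; It also caches a BP_TurretDemo reference, unused here.
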(event OnComponentBeginOverlap(Speed)
  (params (OverlappedComponent :type Primitive%20Component%20Object%20Reference) (OtherActor :type Actor%20Object%20Reference) (OtherComp :type Primitive%20Component%20Object%20Reference) (OtherBodyIndex :type Integer) (bFromSweep :type Boolean) (SweepResult :type Hit%20Result%20Structure%20%28by%20ref%29))
  (Utilities|Casting|CastToBP_SpaceDemo OtherActor)
  (Components|Timeline|SetPlayRate (Variables|Default|GetTimeline) (/ 1.0 15.0)))

(event OnComponentBeginOverlap(Slow)
  (params (OverlappedComponent :type Primitive%20Component%20Object%20Reference) (OtherActor :type Actor%20Object%20Reference) (OtherComp :type Primitive%20Component%20Object%20Reference) (OtherBodyIndex :type Integer) (bFromSweep :type Boolean) (SweepResult :type Hit%20Result%20Structure%20%28by%20ref%29))
  (Utilities|Casting|CastToBP_SpaceDemo OtherActor)
  (Components|Timeline|SetPlayRate (Variables|Default|GetTimeline) (/ 1.0 1e+02)))

(event Custom|PlayTimeLine
  (bind _spline (Variables|Default|GetSpline))
  (bind _returnvalue (Spline|GetSplineLength _spline))
  ;[1 1 1] Starting Timeline
  (bind _alpha_2 (Timeline|Timeline Play)
    (:Update
      (for (_array_element _array_index) (Variables|Default|GetActors)
        (bind _output_get (Variables|Default|SetDistanceAlongSpline (+ (Math|Float|Lerp 0.0 (Spline|GetSplineLength (Variables|Default|GetSpline)) _alpha_2) (* _array_index (Variables|Default|GetOffsetbetweenActors)))))
        (if (> _output_get _returnvalue)
          (Variables|Default|SetDistanceAlongSpline (- (Variables|Default|GetDistanceAlongSpline) _returnvalue))
          (else
            (Transformation|SetActorLocationAndRotation _array_element (Spline|GetLocationatDistanceAlongSpline (Variables|Default|GetSpline) (Variables|Default|GetDistanceAlongSpline) "World") (Spline|GetRotationatDistanceAlongSpline (Variables|Default|GetSpline) (Variables|Default|GetDistanceAlongSpline) "World"))))))))

(event EventBeginPlay
  (Components|Timeline|SetPlayRate (Variables|Default|GetTimeline) (/ 1.0 (Variables|Default|GetTimelineLength)))
  (CallFunction|PlayTimeLine)
  (bind _returnvalue (Actor|GetActorOfClass "/Game/01-Blueprints/Hover/AllHovers/BP_TurretDemo.BP_TurretDemo_C"))
  (Variables|Default|SetBP_TurretDemo _returnvalue))

(fn ConstructionScript
  ;[1 1 1] Récupère les actors de la splines
  (for (_array_element _array_index) (Variables|Default|GetActors)
    (Transformation|SetActorLocationAndRotation _array_element (Spline|GetLocationatDistanceAlongSpline (Variables|Default|GetSpline) (* (Variables|Default|GetOffsetbetweenActors) _array_index) "World") (Spline|GetRotationatDistanceAlongSpline (Variables|Default|GetSpline) (* (Variables|Default|GetOffsetbetweenActors) _array_index) "World"))))