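; BP_Personnalisation sets up the spacecraft customization screen when play begins.
; It creates the WG_Personnalisation widget, shows the mouse cursor, and caches the showroom hover controller and the BP_SauvegardePersonnalisation save actor found in the level.
; After a short delay, it has the save actor load meshes into the Spacecraft_Player data asset, then calls SetupPosForEachMeshPart to position the mesh parts.
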(event EventBeginPlay
  (bind _returnvalue (Game|ConstructObjectfromClass "/Game/05-UI/WG_Personnalisation.WG_Personnalisation_C"))
  (bind _output_get (Variables|Default|SetWG_Personnalisation _returnvalue))
  (UserInterface|Viewport|AddtoViewport _output_get 0)
  (Variables|/Script/Engine.PlayerController|SetbShowMouseCursor (Game|GetPlayerController 0) true)
  (bind _returnvalue_2 (Actor|GetActorOfClass "/Game/01-Blueprints/Hover/Showroom/BP_HoverControllerShowRoom.BP_HoverControllerShowRoom_C"))
  (Variables|Default|SetHoverControllerShowRoom _returnvalue_2)
  (bind _returnvalue_3 (Actor|GetActorOfClass "/Game/01-Blueprints/Sauvegarde/BP_SauvegardePersonnalisation.BP_SauvegardePersonnalisation_C"))
  (bind _output_get_2 (Variables|Default|SetSauvegardePersonnalisation _returnvalue_3))
  (Utilities|FlowControl|Delay 0.1)
  (Class|SauvegardePersonnalisation|LoadMeshtoTargetDataAsset _output_get_2 "/Game/01-Blueprints/Spacecraft/DataAssets/Spacecraft_Player.Spacecraft_Player" self)
  (Class|Personnalisation|SetupPosforEachMeshPart))

(fn ConstructionScript)