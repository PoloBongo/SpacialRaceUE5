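; Checkpoint actor that records a hover controller's progress through numbered checkpoints in sequence.
; Three seconds after BeginPlay it caches the first BP_HoverController found, which receives all updates regardless of which hover controller overlaps the box.
; An overlap counts only if this index follows LastCp, marking the LastCp slot in CpPassed before advancing LastCp.
; A DoOnce with a five-second delayed reset debounces repeat overlaps.
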(event OnComponentBeginOverlap(Box)
  (params (OverlappedComponent :type Primitive%20Component%20Object%20Reference) (OtherActor :type Actor%20Object%20Reference) (OtherComp :type Primitive%20Component%20Object%20Reference) (OtherBodyIndex :type Integer) (bFromSweep :type Boolean) (SweepResult :type Hit%20Result%20Structure%20%28by%20ref%29))
  (bind _checkpointindex (Variables|Default|GetCheckPointIndex))
  (bind _refplayer (Variables|Default|GetRefPlayer))
  (Utilities|Casting|CastToBP_HoverController OtherActor)
  (Utilities|FlowControl|DoOnce false :!label _label
    (:Completed
      (if (== _checkpointindex (+ (Variables|/Game/01-Blueprints/Hover/BP_HoverController.BP_HoverController_C|GetLastCp _refplayer) 1))
        (Utilities|Array|SetArrayElem (Variables|/Game/01-Blueprints/Hover/BP_HoverController.BP_HoverController_C|GetCpPassed _refplayer) (Variables|/Game/01-Blueprints/Hover/BP_HoverController.BP_HoverController_C|GetLastCp _refplayer) true)
        (Variables|/Game/01-Blueprints/Hover/BP_HoverController.BP_HoverController_C|SetLastCp _refplayer _checkpointindex))
      (Utilities|FlowControl|Delay 5.0)
      (goto _label Reset))))

(event EventBeginPlay
  (Utilities|FlowControl|Delay 3.0)
  (bind _returnvalue (Actor|GetActorOfClass "/Game/01-Blueprints/Hover/BP_HoverController.BP_HoverController_C"))
  (Variables|Default|SetRefPlayer _returnvalue))

(fn ConstructionScript)